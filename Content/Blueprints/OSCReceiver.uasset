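; OSCReceiver is an actor Blueprint that receives two float values, treated as X and Y, over OSC.
; On BeginPlay it starts a listening OSC server on a hardcoded IP and port, clears bundle-received bindings and binds a message-received event.
; The message handler, which does not filter by OSC address, stores the first two floats in ValueX and ValueY and prints them for debugging.
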(event `self.ReceiveBeginPlay`
  (bind _returnvalue (`OSCManager.CreateOSCServer` "192.168.178.29" 8080 false true "" null))
  (bind _output_get (set `self.OSCServer` _returnvalue))
  (clear `OSCServer.OnOscBundleReceived` _output_get)
  (add `OSCServer.OnOscMessageReceived` _output_get (`|CreateDelegate` :!event `OSCMessageRecived`)))

(event `OSCMessageRecived`
  (params (Message :type "OSCMessage Structure (by ref)") (IPAddress :type String) (Port :type Integer))
  (bind _value (`OSCManager.GetFloat` Message))
  (bind _output_get (set `self.ValueX` _value))
  (bind _value_2 (`OSCManager.GetFloat` Message 1))
  (bind _output_get_2 (set `self.ValueY` _value_2))
  (`KismetSystemLibrary.PrintString` (`KismetStringLibrary.Concat_StrStr` "Index 0 (x) = " (`KismetStringLibrary.Conv_DoubleToString` _output_get) "  +  " "Index 1 (y) = " (`KismetStringLibrary.Conv_DoubleToString` _output_get_2))))

(fn `UserConstructionScript`)